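; Tank pawn with an independently aimed turret that fires color-matched bouncing rockets on a cooldown.
; A controller-set heading turns the head each tick, while movement vectors rotate the body and drive it along its forward axis, dampening velocity by turn angle.
; Rocket stats come from the owning game container's rocket types.
; Hits, except self-hits just after firing, spawn explosion effects, report the kill to that container and expire the pawn.
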(event `self.ReceiveTick`
  (params (DeltaSeconds :type "Float (single-precision)"))
  ;[1 1 1] Event Tick: being used to rotate the turret to the input heading, and to calculate cooldown left
  (`|ExecutionSequence`
    (:`then_0`
      (if (> (`self.RemainingRocketCooldown`) 0.0)
        (set `self.RemainingRocketCooldown` (- (`self.RemainingRocketCooldown`) DeltaSeconds))))
    (:`then_1`
      (`KismetSystemLibrary.MoveComponentTo` (`self.TankHead`) (0.0 0.0 22.875724) (`KismetMathLibrary.MakeRotator` 0.0 0.0 (`self.CurrentHeading`)) false false (`self.Tank Aim Snappiness`) true))))

(event `Play Tank Movement Sound`
  (bind _tankmovementsound (`self.TankMovementSound`))
  ;[1 1 1] Handle Tank Movement Sounds
  (if (not (`AudioComponent.IsPlaying` _tankmovementsound))
    (`AudioComponent.FadeIn` _tankmovementsound 0.5 1.0 0.0 "Linear")))

(event `Stop Tank Movement Sound`
  ;[1 1 1] Handle Tank Movement Sounds
  (`AudioComponent.FadeOut` (`self.TankMovementSound`) 0.3 0.0 "Linear"))

(event `self.ReceiveBeginPlay`
  ;[1 1 1] On tank spawn, set the tank color
  (`self.Set Up Material Instances`)
  (`self.Set Tank Color` (`self.TankColor`) (`self.DefaultColorStrength`)))

(event `On Hit`
  (params (`Origin Tank ID` :type Integer))
  (bind _returnvalue (`self.K2_GetActorLocation`))
  ;[1 1 1] Event that runs when the tank is hit by a projectile
  (if (not (and (< (- (`self.RocketCooldown`) (`self.RemainingRocketCooldown`)) 0.1) (== `Origin Tank ID` (`self.TankId`))))
    (`|ExecutionSequence`
      (:`then_0`
        (`NiagaraFunctionLibrary.SpawnSystemAtLocation` "/Game/WiiTainks_Content/Game/FX/FXSystem_TankExplosion.FXSystem_TankExplosion" _returnvalue)
        (`GameplayStatics.SpawnSoundAtLocation` "/Game/WiiTainks_Content/Tanks/Sounds/TankExplosion_Cue.TankExplosion_Cue" _returnvalue (struct) 1.0 1.0 0.0 null null))
      (:`then_1`
        (`/Game/WiiTainks_Content/Game/BP_WiiTainks_GameContainer.Tank Destroyed` (`self.Owner Game Container`) (`self.TankId`) `Origin Tank ID`)
        (`self.SetLifeSpan` 0.1)))))

(event `self.ReceivePossessed`
  (params (NewController :type "Controller Object Reference"))
  (bind _max_movement_speed (`self.Max Movement Speed`))
  (bind _floatingpawnmovement (`self.FloatingPawnMovement`))
  ;[1 1 1] Set tank speed on possession
  (set `FloatingPawnMovement.MaxSpeed` _max_movement_speed _floatingpawnmovement)
  (set `FloatingPawnMovement.Acceleration` _max_movement_speed _floatingpawnmovement)
  (set `FloatingPawnMovement.Deceleration` (* _max_movement_speed 3.0) _floatingpawnmovement)
  (`self.Initialize Movement Values`))

(event `Move Tank By Egocentric Vector`
  (params (`TankHead Centric Vector` :type "Vector2D Structure"))
  ;[1 1 1] Move Action trigger, but converts egocentric direction vector into usable world direction vector)
  (`self.Move Tank By World Vector` (`self.Convert Egocentric Direction Vector to World Unit Vector` `TankHead Centric Vector`)))

(event `Move Tank By World Vector`
  (params (`Direction Vector` :type "Vector2D Structure"))
  (bind _floatingpawnmovement (`self.FloatingPawnMovement`))
  (bind _returnvalue (`SceneComponent.GetForwardVector` (`self.Tank Body`)))
  (bind _returnvalue_2 (`KismetMathLibrary.VSize2D` (`self.Convert XY Direction Vector to Radial Vector (Normalize Magnitude)` `Direction Vector`)))
  (bind _returnvalue_3 (`KismetMathLibrary.RadiansToDegrees` (`KismetMathLibrary.Vector_HeadingAngle` (`KismetMathLibrary.Conv_Vector2DToVector` `Direction Vector`))))
  (bind _returnvalue_4 (`KismetMathLibrary.Abs` (`self.Get Heading Degree Difference` _returnvalue_3 (`KismetMathLibrary.RadiansToDegrees` (`KismetMathLibrary.Vector_HeadingAngle` _returnvalue)))))
  ;[1 1 1] Move Tank: this is the logic for taking in a directional vector and using it to apply movement
  (`self.Play Tank Movement Sound`)
  (set `MovementComponent.Velocity` (`self.Tank Velocity Dampener` (`MovementComponent.Velocity` _floatingpawnmovement) (`self.Tank Turning Dampening Factor`) _returnvalue_4) _floatingpawnmovement)
  (`PawnMovementComponent.AddInputVector` (`self.FloatingPawnMovement`) (* _returnvalue_2 _returnvalue) false)
  (`KismetSystemLibrary.MoveComponentTo` (`self.Tank Body`) (0.0 0.0 -38.893689) (`KismetMathLibrary.MakeRotator` 0.0 0.0 _returnvalue_3) false false (`self.Tank Turn Time Calculator` _returnvalue_2 _returnvalue_4) :!label _label))

(event `Stop Tank Rotation`
  ;[1 1 1] Move Tank: this is the logic for taking in a directional vector and using it to apply movement
  (`self.Stop Tank Movement Sound`)
  (`KismetSystemLibrary.Delay` (/ (`self.Tank Turn Time`) 2.0))
  (goto _label :!via `Stop`))

(event `Shoot Action`
  (params (`Direction Vector` :type "Vector Structure"))
  (bind _returnvalue (`SceneComponent.K2_GetComponentToWorld` (`self.BarrelEnd`)))
  ;[1 1 1] Perform Shoot Action (shoots wherever the turret barrel is aimed when triggered)
  (if (<= (`self.RemainingRocketCooldown`) 0.0)
    (`ActorComponent.Activate` (`self.Niagara`) false)
    (`|SpawnActorFromClass` "/Game/WiiTainks_Content/Tanks/Blueprints/BP_Rocket.BP_Rocket_C" (`KismetMathLibrary.MakeTransform` (.location _returnvalue) (`KismetMathLibrary.MakeRotator` 0.0 0.0 (.yaw (.rotation _returnvalue))) (1.2 1.2 1.2)) "AlwaysSpawn" "MultiplyWithRoot" self (`self.Rocket Max Bounces`) (`self.TankId`) (`self.RocketSpeed`) (`self.TankColor`) null)
    (`GameplayStatics.PlaySound2D` "/Game/WiiTainks_Content/Tanks/Sounds/TankFire_Cue.TankFire_Cue" 1.0 1.0 0.0 null null false)
    (set `self.RemainingRocketCooldown` (`self.RocketCooldown`))))

(fn `Initialize Movement Values`
  (set `self.Tank Turn Time` (- 1.0 (/ (`self.Max Movement Speed`) 1000.0)))
  (set `self.Tank Turning Dampening Factor` (`KismetMathLibrary.FClamp` (- 100.0 (/ (`self.Max Movement Speed`) 3.5294)) 1.0 100.0)))

(fn `Set Rocket Type`
  (params (`Rocket Type Index` :type Integer))
  (returns (`New Max Bounces` :type Integer) (`New Rocket Speed` :type "Float (double-precision)") (`New Cooldown Time` :type "Float (double-precision)"))
  (bind (_output_rocketmaxbounces _output_rocketspeed _output_cooldowntime) (break `/Game/WiiTainks_Content/Tanks/Blueprints/Structs/RocketType` (`|GetArrayItem` (`/Game/WiiTainks_Content/Game/BP_WiiTainks_GameContainer.RocketTypes` (`self.Owner Game Container`)) `Rocket Type Index`)))
  (set `self.Rocket Max Bounces` _output_rocketmaxbounces)
  (bind _output_get (set `self.RocketCooldown` _output_cooldowntime))
  (bind _output_get_2 (set `self.RocketSpeed` _output_rocketspeed))
  (return _output_rocketmaxbounces _output_get_2 _output_get))

(fn `Set Tank Color`
  (params (`New Color` :type "LinearColor Structure") (`Color Strength` :type "Float (double-precision)"))
  (locals (`New Color Input` :type "LinearColor Structure") (`New Color Strength` :type "Float (double-precision)"))
  (bind _new_color_input (`local.New Color Input`))
  (bind _new_color_strength (`local.New Color Strength`))
  (set `local.New Color Strength` `Color Strength`)
  (set `local.New Color Input` `New Color`)
  (`MaterialInstanceDynamic.SetVectorParameterValue` (`self.TankMetal_MaterialInstance`) "NewColor" _new_color_input)
  (`MaterialInstanceDynamic.SetVectorParameterValue` (`self.TankMetal2_MaterialInstance`) "NewColor" _new_color_input)
  (`MaterialInstanceDynamic.SetScalarParameterValue` (`self.TankMetal_MaterialInstance`) "ColorStrength" _new_color_strength)
  (`MaterialInstanceDynamic.SetScalarParameterValue` (`self.TankMetal2_MaterialInstance`) "ColorStrength" _new_color_strength))

(fn `Set Up Material Instances`
  (bind _returnvalue (`KismetMaterialLibrary.CreateDynamicMaterialInstance` "/Game/WiiTainks_Content/Tanks/Materials/TankMetal.TankMetal"))
  (bind _output_get (set `self.TankMetal_MaterialInstance` _returnvalue))
  (`PrimitiveComponent.SetMaterial` (`self.Tank Body`) 0 _output_get)
  (bind _returnvalue_2 (`KismetMaterialLibrary.CreateDynamicMaterialInstance` "/Game/WiiTainks_Content/Tanks/Materials/TankMetal2.TankMetal2"))
  (bind _output_get_2 (set `self.TankMetal2_MaterialInstance` _returnvalue_2))
  (`PrimitiveComponent.SetMaterial` (`self.TankHead`) 0 _output_get_2))

(fn `Update Heading`
  (params (`New Heading` :type "Float (double-precision)"))
  (set `self.CurrentHeading` `New Heading`))

(fn `UserConstructionScript`)