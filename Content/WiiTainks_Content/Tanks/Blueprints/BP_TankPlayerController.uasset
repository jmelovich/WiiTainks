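; Player controller for the tank game, translating Enhanced Input into move, turret, shoot and rocket-type actions on the possessed BP_TankPawn.
; A looping timer aims the turret at the mouse cursor until directional rotate input takes over; mouse clicks switch back.
; Assigning a game container sets the view target and creates the overlay, which shows rocket cooldown and bounce count.
; Scroll input cycles the container's rocket types with a short debounce.
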(event `self.ReceiveBeginPlay`
  ;[1 1 1] Set up references and add mapping context (to allow for player input to be recieved)
  (`EnhancedInputSubsystemInterface.AddMappingContext` (pcsubsystem `EnhancedInputLocalPlayerSubsystem` self) "/Game/WiiTainks_Content/Tanks/Input/IMC_PlayerMappings.IMC_PlayerMappings" 0 (struct)))

(event `self.ReceiveTick`
  (params (DeltaSeconds :type "Float (single-precision)"))
  (`self.UpdateRemainingCooldownUI`))

(event `self.ReceiveUnPossess`
  (params (UnpossessedPawn :type "Pawn Object Reference"))
  ;[1 1 1] Possession Event, begin updating turret rotation
  (`KismetSystemLibrary.K2_ClearAndInvalidateTimerHandle` (stale `self.ReceivePossess` _returnvalue)))

(event `self.ReceivePossess`
  (params (PossessedPawn :type "Pawn Object Reference"))
  (bind _gameoverlayui (`self.GameOverlayUI`))
  ;[1 1 1] Possession Event, begin updating turret rotation
  (bind _asbp_tank_pawn (cast `/Game/WiiTainks_Content/Tanks/Blueprints/BP_TankPawn` PossessedPawn))
  (bind _output_get (set `self.Tank Pawn` _asbp_tank_pawn))
  (`|ExecutionSequence`
    (:`then_0`
      (bind _returnvalue (`KismetSystemLibrary.K2_SetTimerDelegate` (delegate `Update Turret By Mouse Position`) 0.05 true)))
    (:`then_1`
      (if (`KismetSystemLibrary.IsValid` _gameoverlayui)
        (set `/Game/WiiTainks_Content/UI/GameOverlay.Current Max Rocket Bounces` (`/Game/WiiTainks_Content/Tanks/Blueprints/BP_TankPawn.Rocket Max Bounces` _output_get) _gameoverlayui)))))

(event `Update Turret By Mouse Position`
  ;[1 1 1] Possession Event, begin updating turret rotation
  (if (`self.isUsingMouseInput`)
    (bind _heading (`self.Get Heading From Mouse Cursor`))
    (`/Game/WiiTainks_Content/Tanks/Blueprints/BP_TankPawn.Update Heading` (`self.Tank Pawn`) _heading)))

(event `EnhancedInput|/Game/WiiTainks_Content/Tanks/Input/Actions/IA_Move`
  (params (ActionValue :type "Vector2D Structure") (ElapsedSeconds :type "Float (double-precision)") (TriggeredSeconds :type "Float (double-precision)") (InputAction :type "InputAction Object Reference" :default "/Game/WiiTainks_Content/Tanks/Input/Actions/IA_Move.IA_Move"))
  (bind _tank_pawn (`self.Tank Pawn`))
  ;[1 1 1] Move Action
  (:`Triggered`
    (`/Game/WiiTainks_Content/Tanks/Blueprints/BP_TankPawn.Move Tank By World Vector` _tank_pawn (`self.Convert Player Input To Game Container Relative` ActionValue)))
  (:`Completed`
    (`/Game/WiiTainks_Content/Tanks/Blueprints/BP_TankPawn.Stop Tank Rotation` _tank_pawn)))

(event `EnhancedInput|/Game/WiiTainks_Content/Tanks/Input/Actions/IA_Shoot`
  (params (ActionValue :type Boolean) (ElapsedSeconds :type "Float (double-precision)") (TriggeredSeconds :type "Float (double-precision)") (InputAction :type "InputAction Object Reference" :default "/Game/WiiTainks_Content/Tanks/Input/Actions/IA_Shoot.IA_Shoot"))
  ;[1 1 1] Shoot Action
  (:`Triggered`
    (`/Game/WiiTainks_Content/Tanks/Blueprints/BP_TankPawn.Shoot Action` (`self.Tank Pawn`) (`.Location` (`GameplayStatics.BreakHitResult` (`self.GetHitResultUnderCursorByChannel` "TraceTypeQuery1"))))))

(event `Key|LeftMouseButton`
  (params (Key :type "Key Structure"))
  ;[1 1 1] For Switching Between Input Types
  (:`Pressed`
    (set `self.isUsingMouseInput` true :!label _label)))

(event `EnhancedInput|/Game/WiiTainks_Content/Tanks/Input/Actions/IA_RotateTurret`
  (params (ActionValue :type "Vector2D Structure") (ElapsedSeconds :type "Float (double-precision)") (TriggeredSeconds :type "Float (double-precision)") (InputAction :type "InputAction Object Reference" :default "/Game/WiiTainks_Content/Tanks/Input/Actions/IA_RotateTurret.IA_RotateTurret"))
  ;[1 1 1] Rotate Turret Action (Used by AI Agents and Gamepad)
  (:`Triggered`
    (set `self.isUsingMouseInput` false)
    (bind _heading (`self.Get Heading From Directional Input` ActionValue))
    (`/Game/WiiTainks_Content/Tanks/Blueprints/BP_TankPawn.Update Heading` (`self.Tank Pawn`) _heading)))

(event `Key|RightMouseButton`
  (params (Key :type "Key Structure"))
  ;[1 1 1] For Switching Between Input Types
  (:`Pressed`
    (goto _label)))

(event `EnhancedInput|/Game/WiiTainks_Content/Tanks/Input/Actions/IA_Scroll`
  (params (ActionValue :type "Float (double-precision)") (ElapsedSeconds :type "Float (double-precision)") (TriggeredSeconds :type "Float (double-precision)") (InputAction :type "InputAction Object Reference" :default "/Game/WiiTainks_Content/Tanks/Input/Actions/IA_Scroll.IA_Scroll"))
  (bind _tank_pawn (`self.Tank Pawn`))
  ;[1 1 1] Scroll Action: cycle between current rocket type
  (:`Triggered`
    (`/Engine/EditorBlueprintResources/StandardMacros.DoOnce` false :!label _label_2
      (:`Completed`
        (bind _new_max_bounces (`/Game/WiiTainks_Content/Tanks/Blueprints/BP_TankPawn.Set Rocket Type` _tank_pawn (`KismetMathLibrary.Clamp` (+ ActionValue (`/Game/WiiTainks_Content/Tanks/Blueprints/BP_TankPawn.Rocket Max Bounces` _tank_pawn)) 0 (`KismetArrayLibrary.Array_LastIndex` (`/Game/WiiTainks_Content/Game/BP_WiiTainks_GameContainer.RocketTypes` (`self.Owner Game Container`))))))
        (set `/Game/WiiTainks_Content/UI/GameOverlay.Current Max Rocket Bounces` _new_max_bounces (`self.GameOverlayUI`))
        (`KismetSystemLibrary.Delay` 0.1)
        (goto _label_2 :!via `Reset`)))))

(fn `Get Heading From Directional Input`
  (params (`Directional Input` :type "Vector2D Structure"))
  (returns (Heading :type "Float (double-precision)"))
  (return (`KismetMathLibrary.RadiansToDegrees` (`KismetMathLibrary.Vector_HeadingAngle` (`KismetMathLibrary.Conv_Vector2DToVector` (`self.Convert Player Input To Game Container Relative` `Directional Input`))))))

(fn `Get Heading From Mouse Cursor`
  (returns (Heading :type "Float (double-precision)"))
  (return (`KismetMathLibrary.RadiansToDegrees` (`KismetMathLibrary.Vector_HeadingAngle` (`KismetMathLibrary.GetDirectionUnitVector` (`self.K2_GetActorLocation` (`self.Tank Pawn`)) (`.Location` (`GameplayStatics.BreakHitResult` (`self.GetHitResultUnderCursorByChannel` "TraceTypeQuery1" false))))))))

(fn `Update Game Container`
  (params (`Game Container` :type "/Game/WiiTainks_Content/Game/BP_WiiTainks_GameContainer Object Reference"))
  (bind _output_get (set `self.Owner Game Container` `Game Container`))
  (`self.SetViewTargetWithBlend` _output_get)
  (`/Engine/EditorBlueprintResources/StandardMacros.IsValid` (`self.GameOverlayUI`)
    (:`Is Not Valid`
      (bind _returnvalue (`|CreateWidget` "/Game/WiiTainks_Content/UI/GameOverlay.GameOverlay_C" self))
      (bind _output_get_2 (set `self.GameOverlayUI` _returnvalue))
      (`UserWidget.AddToPlayerScreen` _output_get_2 0))))

(fn `UpdateRemainingCooldownUI`
  (bind _gameoverlayui (`self.GameOverlayUI`))
  (if (`KismetSystemLibrary.IsValid` _gameoverlayui)
    (set `/Game/WiiTainks_Content/UI/GameOverlay.Remaining Cooldown Time` (`KismetMathLibrary.FClamp` (`/Game/WiiTainks_Content/Tanks/Blueprints/BP_TankPawn.RemainingRocketCooldown` (`self.Tank Pawn`)) 0.0 99.0) _gameoverlayui)))

(fn `UserConstructionScript`)