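; Bouncing rocket projectile fired by tanks, tinted per shot through a dynamic material instance.
; BeginPlay drives the capsule with ProjectileMovement and briefly delays lethality, while Tick orients the capsule from its velocity.
; Once armed, tank hits, including the owner, call the tank's OnHit and destroy the rocket.
; Other hits count bounces until MaxBounces is exceeded, then spawn explosion effects and sound and destroy it.
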(event `self.ReceiveBeginPlay`
  (bind _projectilemovement (`self.ProjectileMovement`))
  (bind _speed (`self.Speed`))
  ;[1 1 1] Begin Play: this runs at spawn to set the collider as projectile movement target, it also sets the color of the rocket (based on the input pin from the tank pawn)
  (`MovementComponent.SetUpdatedComponent` (`self.ProjectileMovement`) (`self.Capsule`))
  (set `ProjectileMovementComponent.InitialSpeed` _speed _projectilemovement)
  (set `ProjectileMovementComponent.MaxSpeed` (* _speed 2.0) _projectilemovement)
  (`self.Set Rocket Color` (`self.Rocket Color`))
  (`KismetSystemLibrary.Delay` 0.1)
  (set `self.canKill` true)
  (`KismetSystemLibrary.Delay` 0.1)
  (`RectLightComponent.SetSourceHeight` (`self.RectLight`) 192.0))

(event `self.ReceiveHit`
  (params (MyComp :type "PrimitiveComponent Object Reference") (Other :type "Actor Object Reference") (OtherComp :type "PrimitiveComponent Object Reference") (bSelfMoved :type Boolean) (HitLocation :type "Vector Structure") (HitNormal :type "Vector Structure") (NormalImpulse :type "Vector Structure") (Hit :type "HitResult Structure (by ref)"))
  (bind (_returnvalue_roll _returnvalue_pitch _returnvalue_yaw) (`KismetMathLibrary.BreakRotator` (`KismetMathLibrary.Conv_VectorToRotator` HitNormal)))
  ;[1 1 1] Event Hit: this runs whenever the rocket hits something
  (bind _asbp_tank_pawn (cast `/Game/WiiTainks_Content/Tanks/Blueprints/BP_TankPawn` Other)
    (:`then`
      (if (`self.canKill`)
        (bind _tankid (`/Game/WiiTainks_Content/Tanks/Blueprints/BP_TankPawn.TankId` _asbp_tank_pawn))
        (if (== (`self.OwnerID`) _tankid)
          (`KismetSystemLibrary.PrintString` "HIT SELF")
          (else
            (`KismetSystemLibrary.PrintText` (`|FormatText` "Hit Tank With ID: {id}" _tankid))))
        (`/Game/WiiTainks_Content/Tanks/Blueprints/BP_TankPawn.On Hit` _asbp_tank_pawn _tankid)
        (`self.K2_DestroyActor` :!label _label)))
    (:`CastFailed`
      (bind _result (`/Engine/EditorBlueprintResources/StandardMacros.IncrementInt` (`self.TotalBounces`))
        (:`  `
          (if (> _result (`self.MaxBounces`))
            (`NiagaraFunctionLibrary.SpawnSystemAtLocation` "/Game/WiiTainks_Content/Game/FX/FXSystem_RocketExplosion.FXSystem_RocketExplosion" HitLocation (`KismetMathLibrary.MakeRotator` 0.0 (`KismetMathLibrary.SelectFloat` 0.0 90.0 (== Other "BP_Rocket")) (+ _returnvalue_yaw 180.0)) (0.1 0.1 0.1))
            (`GameplayStatics.SpawnSoundAtLocation` "/Game/WiiTainks_Content/Tanks/Sounds/RocketExplosion_Cue.RocketExplosion_Cue" HitLocation (struct) 1.0 1.0 0.0 null null)
            (goto _label)))))))

(event `self.ReceiveTick`
  (params (DeltaSeconds :type "Float (single-precision)"))
  (bind _capsule (`self.Capsule`))
  (bind (_returnvalue_roll _returnvalue_pitch) (`KismetMathLibrary.BreakRotator` (`SceneComponent.K2_GetComponentRotation` _capsule)))
  (bind (_returnvalue_roll_2 _returnvalue_pitch_2 _returnvalue_yaw) (`KismetMathLibrary.BreakRotator` (`KismetMathLibrary.Conv_VectorToRotator` (`SceneComponent.GetComponentVelocity` _capsule))))
  ;[1 1 1] Event Tick: this runs each frame and orients the projectile based on its velocity vector
  (`SceneComponent.K2_SetWorldRotation` _capsule (`KismetMathLibrary.MakeRotator` _returnvalue_yaw _returnvalue_pitch) false false))

(fn `Set Rocket Color`
  (params (`New Rocket Color` :type "LinearColor Structure"))
  (bind _returnvalue (`KismetMaterialLibrary.CreateDynamicMaterialInstance` "/Game/WiiTainks_Content/Tanks/Materials/BareMetal.BareMetal"))
  (`MaterialInstanceDynamic.SetVectorParameterValue` _returnvalue "NewColor" (`local.New Rocket Color`))
  (`MaterialInstanceDynamic.SetScalarParameterValue` _returnvalue "ColorStrength" (`self.Rocket Color Strength`))
  (`PrimitiveComponent.SetMaterial` (`self.RocketMesh`) 0 _returnvalue))

(fn `UserConstructionScript`)