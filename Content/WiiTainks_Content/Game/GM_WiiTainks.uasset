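; GM_WiiTainks, by its name the WiiTainks game mode, tracks the game containers in the level and resolves which one owns a given tank.
; BeginPlay caches every BP_WiiTainks_GameContainer actor.
; GetOwningGameContainer casts the passed actor to BP_TankPawn, then returns the first container that reports holding its TankId, printing an error if none does.
; The lookup matches by ID; the tank location it reads goes unused.
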(event `self.ReceiveBeginPlay`
  ;[1 1 1] Get a list of all game containers in the scene
  (bind _outactors (`GameplayStatics.GetAllActorsOfClass` "/Game/WiiTainks_Content/Game/BP_WiiTainks_GameContainer.BP_WiiTainks_GameContainer_C"))
  (set `self.Game Containers` _outactors))

(fn `GetOwningGameContainer`
  (params (`Actor To Get Container Of` :type "Actor Object Reference"))
  (returns (`Game Container` :type "/Game/WiiTainks_Content/Game/BP_WiiTainks_GameContainer Object Reference"))
  (locals (`Input Actor Location` :type "Vector Structure" :default (0.0 0.0 0.0)) (TankPawn :type "/Game/WiiTainks_Content/Tanks/Blueprints/BP_TankPawn Object Reference"))
  ;[1 1 1] This function gets the owning game container of a passed in tank pawn
  (bind _asbp_tank_pawn (cast `/Game/WiiTainks_Content/Tanks/Blueprints/BP_TankPawn` `Actor To Get Container Of`))
  (bind _output_get (set `local.TankPawn` _asbp_tank_pawn))
  (set `local.Input Actor Location` (`self.K2_GetActorLocation` _output_get))
  (for _array_element (`self.Game Containers`)
    (bind _tank_is_in_container (`/Game/WiiTainks_Content/Game/BP_WiiTainks_GameContainer.Is Tank In Container?` _array_element (`/Game/WiiTainks_Content/Tanks/Blueprints/BP_TankPawn.TankId` (`local.TankPawn`))))
    (if _tank_is_in_container
      (return _array_element)))
  (`KismetSystemLibrary.PrintString` "FAILED TO GET GAME CONTAINER" true true (struct :`R` 1.0 :`A` 1.0) 5.0)
  (return null))

(fn `UserConstructionScript`)