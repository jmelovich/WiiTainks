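; Game container actor for a WiiTainks arena, managing its layout, camera and tanks.
; Construction sizes the bounds, adds four cube walls and places the camera to suit ArenaSize.
; BeginPlay registers nearby tanks, optionally scatters obstacles from a seeded random stream over a flattened square grid, then spawns and possesses the player's tank.
; Destroyed tanks respawn immediately at a random grid cell with the same ID, color and controller, as placeholder game logic.
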(event `self.ReceiveBeginPlay`
  (bind _gen_seed (`self.Gen_Seed`))
  ;[1 1 1] Begin Play: this runs whenever the game starts or the container spawns
  (`|ExecutionSequence`
    (:`then_0`
      (`self.Update Tank References`)
      (`KismetSystemLibrary.PrintString` "Updated Tank References"))
    (:`then_1`
      (bind _asgm_wii_tainks (cast `/Game/WiiTainks_Content/Game/GM_WiiTainks` (`GameplayStatics.GetGameMode`)))
      (set `self.WiiTainks_GameMode` _asgm_wii_tainks))
    (:`then_2`
      (`self.Generate Arena` (`KismetMathLibrary.SelectInt` (`KismetMathLibrary.RandomInteger` 9999) _gen_seed (< _gen_seed 0)))
      (bind _spawnable_transform (`self.Get Available Location In Bounds`))
      (bind _spawned_tank (`self.Spawn New Tank` 0 _spawnable_transform (`self.Player Tank Color`)))
      (`self.Possess Tank` (`GameplayStatics.GetPlayerController` 0) _spawned_tank))))

(event `self.K2_OnBecomeViewTarget`
  (params (PC :type "PlayerController Object Reference"))
  (bind _playercamera (`self.PlayerCamera`))
  ;[1 1 1] This runs when the container is switched to, to make sure the correct camera is set
  (set `self.Player Controller` PC)
  (`ActorComponent.SetActive` _playercamera true true)
  (`ActorComponent.Activate` _playercamera true))

(event `Tank Destroyed`
  (params (`Tank ID` :type Integer))
  ;[1 1 1] This Event is called whenever a tank is destroyed
  (bind (_empty_controller _tank_color) (`self.Handle Tank Destroyed` `Tank ID`))
  (`|ExecutionSequence`
    (:`then_0`
      (bind _spawnable_transform (`self.Get Available Location In Bounds`))
      (bind _spawned_tank (`self.Spawn New Tank` `Tank ID` _spawnable_transform _tank_color)))
    (:`then_1`
      (`self.Possess Tank` _empty_controller _spawned_tank))))

(fn `Generate Arena`
  (params (Seed :type Integer))
  (locals (`Grid Divisions` :type Integer :default 0) (RandomStream :type "RandomStream Structure") (`Min Obstacles` :type Integer :default 5) (`Obstacle Count` :type Integer :default 0) (`Obstacle Grid Array` :type "Array of /Game/WiiTainks_Content/Game/BP_Obstacle Object Reference") (`Used Grid Points` :type "Array of Vector2D Structure") (GridArray :type "Array of Integer"))
  (bind _grid_divisions (`local.Grid Divisions`))
  (bind _obstaclescale (`self.ObstacleScale`))
  (bind _randomstream (`local.RandomStream`))
  (bind _returnvalue (- (`local.Grid Divisions`) 1))
  (bind _returnvalue_2 (`KismetMathLibrary.MakeVector2D` (`KismetMathLibrary.Conv_IntToDouble` (`KismetMathLibrary.RandomIntegerInRangeFromStream` _randomstream 0 _returnvalue)) (`KismetMathLibrary.Conv_IntToDouble` (`KismetMathLibrary.RandomIntegerInRangeFromStream` _randomstream 0 _returnvalue))))
  (if (`self.Generate Level Grid?`)
    (set `local.RandomStream` (`KismetMathLibrary.MakeRandomStream` Seed))
    (bind _output_get (set `local.Grid Divisions` (/ (`KismetMathLibrary.Round` (* (`self.ArenaSize`) (`self.Grid Resolution`))) 10)))
    (`self.Initialize Grid Array` _output_get
      (:`Exec Out`
        (set `self.ObstacleScale` (/ (/ (`self.ArenaSize`) (`local.Grid Divisions`)) 50.0))
        (`|ExecutionSequence`
          (:`then_0`
            ;[1 1 1] First we need to calculate the obstacle count we want
            (set `local.Obstacle Count` (`KismetMathLibrary.RandomIntegerInRangeFromStream` (`local.RandomStream`) (`local.Min Obstacles`) (`KismetMathLibrary.FTrunc` (/ (* (* _grid_divisions _grid_divisions) (- 1.0 (`self.Grid Resolution`))) 2.0)))))
          (:`then_1`
            ;[1 1 1] for now, i will use complete randomness to generate (this is where algorithm will go)
            (for _ (range 1 (+ (`local.Obstacle Count`) 1))
              (if (== (`self.Get At (Grid Array)` _returnvalue_2) 0)
                (`self.Set At (Grid Array)` _returnvalue_2 1))))
          (:`then_2`
            ;[1 1 1] spawn in obstacles from grid
            (for (_ _array_index) (`self.2D Grid Array`)
              (bind _coordinates (`self.Get Coords From Index (Grid Array)` _array_index))
              (if (== (`self.Get At (Grid Array)` _coordinates) 1)
                (bind (_world_location _world_rotation) (`self.Calculate World Position from Grid Coords (Grid Array)` _coordinates (`local.Grid Divisions`) _obstaclescale))
                (bind _returnvalue_3 (`|SpawnActorFromClass` "/Game/WiiTainks_Content/Game/BP_Obstacle.BP_Obstacle_C" (`KismetMathLibrary.MakeTransform` _world_location _world_rotation) "Undefined" "MultiplyWithRoot" null _obstaclescale null))
                (`KismetArrayLibrary.Array_Add` (`local.Obstacle Grid Array`) _returnvalue_3)))))))))

(fn `Get Available Location In Bounds`
  (returns (`Spawnable Transform` :type "Transform Structure"))
  (locals (CurrentRandInt :type Integer) (LoopStopper :type Integer))
  (bind _coordinates (`self.Get Coords From Index (Grid Array)` (stale _output_get)))
  (bind _grid_array_entry_value (`self.Get At (Grid Array)` _coordinates))
  (while (or (!= _grid_array_entry_value 0) (< (`local.LoopStopper`) 100))
    (bind _output_get (set `local.CurrentRandInt` (`KismetMathLibrary.RandomIntegerInRange` 0 (- (`KismetArrayLibrary.Array_Length` (`self.2D Grid Array`)) 1))))
    (`/Engine/EditorBlueprintResources/StandardMacros.IncrementInt` (`local.LoopStopper`)))
  (bind (_x _y) (`KismetMathLibrary.BreakVector2D` _coordinates))
  (`KismetSystemLibrary.PrintText` (`|FormatText` "Index: {i}, Coords: ({c1},{c2}), Grid Val: {g}" _output_get _x _y _grid_array_entry_value) true true (struct :`G` 0.66 :`B` 1.0 :`A` 1.0) 15.0)
  (bind (_world_location _world_rotation) (`self.Calculate World Position from Grid Coords (Grid Array)` _coordinates (`KismetMathLibrary.FTrunc` (`KismetMathLibrary.Sqrt` (`KismetMathLibrary.Conv_IntToDouble` (`KismetArrayLibrary.Array_Length` (`self.2D Grid Array`))))) (`self.ObstacleScale`)))
  (return (`KismetMathLibrary.MakeTransform` _world_location _world_rotation)))

(fn `Handle Tank Destroyed`
  (params (`Tank ID` :type Integer))
  (returns (`Empty Controller` :type "Controller Object Reference") (`Tank Color` :type "LinearColor Structure"))
  (locals (`Now Empty Controller` :type "Controller Object Reference") (`Tank Color Out` :type "LinearColor Structure"))
  (bind _tanksincontainer (`self.TanksInContainer`))
  (for (_array_element _array_index) _tanksincontainer
    (if (== (`/Game/WiiTainks_Content/Tanks/Blueprints/BP_TankPawn.TankId` _array_element) `Tank ID`)
      (bind _output_get (set `local.Now Empty Controller` (`Pawn.GetController` _array_element)))
      (`Controller.UnPossess` _output_get)
      (set `local.Tank Color Out` (`/Game/WiiTainks_Content/Tanks/Blueprints/BP_TankPawn.TankColor` _array_element))
      (`KismetArrayLibrary.Array_Remove` _tanksincontainer _array_index)
      (break)))
  (return (`local.Now Empty Controller`) (`local.Tank Color Out`)))

(fn `Initialize Tank Pawn`
  (params (`Tank Pawn` :type "/Game/WiiTainks_Content/Tanks/Blueprints/BP_TankPawn Object Reference"))
  (set `/Game/WiiTainks_Content/Tanks/Blueprints/BP_TankPawn.Game Mode` (`self.WiiTainks_GameMode`) `Tank Pawn`)
  (set `/Game/WiiTainks_Content/Tanks/Blueprints/BP_TankPawn.Owner Game Container` self `Tank Pawn`))

(fn `Is Tank In Container?`
  (params (`Tank Id` :type Integer))
  (returns (`Tank Is In Container` :type Boolean))
  (for _array_element (`self.TanksInContainer`)
    (bind _returnvalue (== (`/Game/WiiTainks_Content/Tanks/Blueprints/BP_TankPawn.TankId` _array_element) `Tank Id`))
    (if _returnvalue
      (return _returnvalue)
      (else
        (`KismetSystemLibrary.PrintString` "Hello"))))
  (return false))

(fn `Possess Tank`
  (params (Controller :type "Controller Object Reference") (`Tank To Control` :type "/Game/WiiTainks_Content/Tanks/Blueprints/BP_TankPawn Object Reference"))
  (`Controller.Possess` Controller `Tank To Control`)
  (bind _asbp_tank_player_controller (cast `/Game/WiiTainks_Content/Tanks/Blueprints/BP_TankPlayerController` Controller))
  (`/Game/WiiTainks_Content/Tanks/Blueprints/BP_TankPlayerController.Update Game Container` _asbp_tank_player_controller self))

(fn `Set Up Arena`
  (params (`New Arena Size` :type "Float (double-precision)"))
  (locals (WallThickness :type "Float (double-precision)" :default 0.4) (WallCoord :type "Float (double-precision)") (CurrentWallLocation :type "Vector Structure" :default (0.0 0.0 0.0)) (CurrentIndex :type Integer) (`Current Wall Scalar` :type "Vector Structure" :default (0.0 0.0 0.0)) (`IsSidewall?` :type Boolean) (WallLength :type "Float (double-precision)"))
  (bind _walllength (`local.WallLength`))
  (bind _arenasize (`self.ArenaSize`))
  (bind _issidewall_ (`local.IsSidewall?`))
  (bind _returnvalue (`KismetMathLibrary.SelectFloat` 0.0 (`local.WallCoord`) (`local.IsSidewall?`)))
  (bind _returnvalue_2 (`KismetMathLibrary.SelectFloat` (`local.WallThickness`) _walllength _issidewall_))
  (bind _returnvalue_3 (`KismetMathLibrary.SelectFloat` (`local.WallCoord`) 0.0 (`local.IsSidewall?`)))
  (bind _returnvalue_4 (> (`local.CurrentIndex`) 2))
  (bind _returnvalue_5 (`KismetMathLibrary.MakeVector` (* _arenasize -1.25) 0.0 (* _arenasize 1.833333)))
  (bind (_returnvalue_roll _returnvalue_pitch) (`KismetMathLibrary.BreakRotator` (`KismetMathLibrary.FindLookAtRotation` _returnvalue_5 (`self.K2_GetActorLocation`))))
  (`BoxComponent.SetBoxExtent` (`self.Game Extents`) (`KismetMathLibrary.MakeVector` `New Arena Size` `New Arena Size` 600.0) true)
  (`|ExecutionSequence`
    (:`then_0`
      (set `local.WallCoord` (+ (* (`local.WallThickness`) 50.0) (`local.New Arena Size`)))
      (set `local.WallLength` (* (`self.ArenaSize`) 0.02)))
    (:`then_1`
      (for _index (range 1 5)
        (set `local.CurrentIndex` _index)
        (set `local.IsSidewall?` (== (mod (`local.CurrentIndex`) 2) 1))
        (`|ExecutionSequence`
          (:`then_0`
            (set `local.CurrentWallLocation` (`KismetMathLibrary.MakeVector` (`KismetMathLibrary.SelectFloat` _returnvalue_3 (* _returnvalue_3 -1.0) _returnvalue_4) (`KismetMathLibrary.SelectFloat` _returnvalue (* _returnvalue -1.0) _returnvalue_4) 25.0)))
          (:`then_1`
            (set `local.Current Wall Scalar` (`KismetMathLibrary.MakeVector` (`KismetMathLibrary.SelectFloat` _returnvalue_2 (+ _returnvalue_2 (* (`local.WallThickness`) 2.0)) (`local.IsSidewall?`)) (`KismetMathLibrary.SelectFloat` _walllength (`local.WallThickness`) _issidewall_) 1.0)))
          (:`then_2`
            (bind _returnvalue_6 (`|AddComponentByClass` "/Script/Engine.StaticMeshComponent" false (`KismetMathLibrary.MakeTransform` (`local.CurrentWallLocation`) (struct) (`local.Current Wall Scalar`))))
            (`StaticMeshComponent.SetStaticMesh` _returnvalue_6 "/Engine/BasicShapes/Cube.Cube")))))
    (:`then_2`
      (`SceneComponent.K2_SetRelativeTransform` (`self.PlayerCamera`) (`KismetMathLibrary.MakeTransform` _returnvalue_5 (`KismetMathLibrary.MakeRotator` 0.0 (* _returnvalue_pitch 1.06))) false false))))

(fn `Spawn New Tank`
  (params (`Tank ID` :type Integer) (`Spawn Transform` :type "Transform Structure") (`Tank Color` :type "LinearColor Structure"))
  (returns (`Spawned Tank` :type "/Game/WiiTainks_Content/Tanks/Blueprints/BP_TankPawn Object Reference"))
  (locals (`New Tank` :type "/Game/WiiTainks_Content/Tanks/Blueprints/BP_TankPawn Object Reference") (`Input Tank ID` :type Integer))
  (bind _new_tank (`local.New Tank`))
  (bind (_output_rocketmaxbounces _output_rocketspeed _output_cooldowntime) (break `/Game/WiiTainks_Content/Tanks/Blueprints/Structs/RocketType` (`|GetArrayItem` (`self.RocketTypes`))))
  (set `local.Input Tank ID` `Tank ID`)
  (bind _returnvalue (`|SpawnActorFromClass` "/Game/WiiTainks_Content/Tanks/Blueprints/BP_TankPawn.BP_TankPawn_C" `Spawn Transform` "AdjustIfPossibleButAlwaysSpawn" "MultiplyWithRoot" null _output_rocketmaxbounces _output_rocketspeed _output_cooldowntime 300.0 `Tank Color` null))
  (bind _output_get (set `local.New Tank` _returnvalue))
  (set `/Game/WiiTainks_Content/Tanks/Blueprints/BP_TankPawn.TankId` (`local.Input Tank ID`) _output_get)
  (`KismetArrayLibrary.Array_Add` (`self.TanksInContainer`) _output_get)
  (`self.Initialize Tank Pawn` _new_tank)
  (return _new_tank))

(fn `Update Tank References`
  (bind _outactors (`GameplayStatics.GetAllActorsOfClass` "/Game/WiiTainks_Content/Tanks/Blueprints/BP_TankPawn.BP_TankPawn_C"))
  (`KismetSystemLibrary.PrintText` (`|FormatText` "Got All Tanks Actors In Level, length: {l}" (`KismetArrayLibrary.Array_Length` _outactors)))
  (`KismetArrayLibrary.Array_Clear` (`self.TanksInContainer`))
  (for _array_element _outactors
    (bind _asbp_tank_pawn (cast `/Game/WiiTainks_Content/Tanks/Blueprints/BP_TankPawn` _array_element))
    (if (`self.Check If Transform is Within Square` (`self.K2_GetActorLocation`) (`self.K2_GetActorLocation` _asbp_tank_pawn) 1200.0)
      (bind _returnvalue (`KismetArrayLibrary.Array_Add` (`self.TanksInContainer`) _asbp_tank_pawn))
      (set `/Game/WiiTainks_Content/Tanks/Blueprints/BP_TankPawn.TankId` _returnvalue _asbp_tank_pawn)
      (`KismetSystemLibrary.PrintText` (`|FormatText` "Added Tank To Container, ID: {id}" (`/Game/WiiTainks_Content/Tanks/Blueprints/BP_TankPawn.TankId` _asbp_tank_pawn)) true true (struct :`G` 0.66 :`B` 1.0 :`A` 1.0) 10.0))))

(fn `UserConstructionScript`
  (`self.Set Up Arena` (`self.ArenaSize`)))