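; BP_RLInferenceManager is an actor that runs a trained Learning Agents neural network for tanks at runtime.
; On BeginPlay it sets up the tank interactor, then binds the tank policy to it with saved policy settings and a network asset.
; Each Tick it runs inference on that policy.
; An unconnected chain that derives tanks per game and grid size from the game mode never runs.
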(event `self.ReceiveBeginPlay`
  (`|ExecutionSequence`
    (:`then_0`
      (`|ExecutionSequence`
        (:`then_0`
          (`LearningAgentsInteractor.SetupInteractor` (`self.BP_TankInteractor`)))
        (:`then_1`
          (`LearningAgentsPolicy.SetupPolicy` (`self.BP_TankPolicy`) (`self.BP_TankInteractor`) (`self.Policy Settings`) "/Game/Learning/DA_TankNetwork_417_hor1.DA_TankNetwork_417_hor1"))))))

(event `self.ReceiveTick`
  (params (DeltaSeconds :type "Float (single-precision)"))
  (`LearningAgentsPolicy.RunInference` (`self.BP_TankPolicy`)))

(fn `UserConstructionScript`)