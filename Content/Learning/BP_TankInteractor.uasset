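; Learning Agents interactor that defines what AI-controlled tanks observe and how their actions drive the tank pawns.
; Observations take egocentric grid and enemy-position arrays from each BP_TankAIController, plus velocity and body angle measured relative to the tank head.
; Actions return turret yaw, throttle and body rotation, applied through the controller and pawn.
; Shooting, rocket and round-time observations, vector movement and game-mode-based array sizing are present but unwired.
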(event `self.ReceiveBeginPlay`)

(event `self.SetupObservations`
  (`|ExecutionSequence`
    (:`then_0`
      (bind _returnvalue (`VectorArrayObservation.AddVectorArrayObservation` null "EgocentricGridArrayObservation" (`self.Grid Array Length`) (`self.VectorScaler`)))
      (set `self.EgocentricGridArrayObservation` _returnvalue))
    (:`then_1`
      (bind _returnvalue_2 (`VectorArrayObservation.AddVectorArrayObservation` null "EnemyTankPositionArrayObservation" (- (`self.Tanks Per Game`) 1) (`self.VectorScaler`)))
      (set `self.EnemyTankPositionArrayObservation` _returnvalue_2))
    (:`then_2`
      (bind _returnvalue_3 (`PlanarVelocityObservation.AddPlanarVelocityObservation` null "TankSelfVelocityObservation"))
      (set `self.TankSelfVelocityObservation` _returnvalue_3)
      (bind _returnvalue_4 (`AngleObservation.AddAngleObservation` null "TankBodyRotationObservation"))
      (set `self.TankBodyRotationObservation` _returnvalue_4))))

(event `self.SetObservations`
  (params (AgentIds :type "Array of Integer (by ref)"))
  (for _array_element AgentIds
    (`|ExecutionSequence`
      (:`then_0`
        (bind _returnvalue (`self.GetAgent` _array_element "/Game/WiiTainks_Content/Tanks/Blueprints/BP_TankAIController.BP_TankAIController_C"))
        (`VectorArrayObservation.SetVectorArrayObservation` (`self.EgocentricGridArrayObservation`) _array_element (`/Game/WiiTainks_Content/Tanks/Blueprints/BP_TankAIController.EgocentricGridArray` _returnvalue))
        (bind _tank_pawn (`/Game/WiiTainks_Content/Tanks/Blueprints/BP_TankAIController.Tank Pawn` _returnvalue))
        (bind _tankhead (`/Game/WiiTainks_Content/Tanks/Blueprints/BP_TankPawn.TankHead` _tank_pawn))
        (`PlanarVelocityObservation.SetPlanarVelocityObservation` (`self.TankSelfVelocityObservation`) _array_element (`Actor.GetVelocity` _tank_pawn) (`SceneComponent.K2_GetComponentRotation` _tankhead))
        (`AngleObservation.SetAngleObservation` (`self.TankBodyRotationObservation`) _array_element (`KismetMathLibrary.Vector_HeadingAngle` (`SceneComponent.GetForwardVector` (`/Game/WiiTainks_Content/Tanks/Blueprints/BP_TankPawn.Tank Body` _tank_pawn))) (`KismetMathLibrary.Vector_HeadingAngle` (`SceneComponent.GetForwardVector` _tankhead))))
      (:`then_1`
        (`VectorArrayObservation.SetVectorArrayObservation` (`self.EnemyTankPositionArrayObservation`) _array_element (`/Game/WiiTainks_Content/Tanks/Blueprints/BP_TankAIController.EgocentricEnemyTanks` _returnvalue))))))

(event `self.SetupActions`
  (`|ExecutionSequence`
    (:`then_1`
      (bind _returnvalue (`RotationAction.AddRotationAction` null "TurretRotatorAction" 1.0))
      (set `self.TurretRotatorAction` _returnvalue)
      (bind _returnvalue_2 (`FloatAction.AddFloatAction` null "MovementThrottleAction" 100.0))
      (set `self.MovementThrottleAction` _returnvalue_2)
      (bind _returnvalue_3 (`RotationAction.AddRotationAction` null "RotationAction" 360.0))
      (set `self.RotationAction` _returnvalue_3))))

(event `self.GetActions`
  (params (AgentIds :type "Array of Integer (by ref)"))
  (for _array_element AgentIds
    (`|ExecutionSequence`
      (:`then_1`
        (bind _returnvalue (`RotationAction.GetRotationAction` (`self.TurretRotatorAction`) _array_element))
        (bind _returnvalue_2 (`self.GetAgent` _array_element "/Game/WiiTainks_Content/Tanks/Blueprints/BP_TankAIController.BP_TankAIController_C"))
        (`/Game/WiiTainks_Content/Tanks/Blueprints/BP_TankAIController.Update Tank Pawn Heading` _returnvalue_2 (* (.yaw _returnvalue) 10.0)))
      (:`then_2`
        (bind _returnvalue_3 (`FloatAction.GetFloatAction` (`self.MovementThrottleAction`) _array_element))
        (`/Game/WiiTainks_Content/Tanks/Blueprints/BP_TankAIController.Move Tank` _returnvalue_2 _returnvalue_3)
        (bind _returnvalue_4 (`RotationAction.GetRotationAction` (`self.RotationAction`) _array_element))
        (`/Game/WiiTainks_Content/Tanks/Blueprints/BP_TankPawn.Rotate Tank Body` (`/Game/WiiTainks_Content/Tanks/Blueprints/BP_TankAIController.Tank Pawn` _returnvalue_2) (.yaw _returnvalue_4))))))