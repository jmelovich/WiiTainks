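; Manager Blueprint that drives Learning Agents reinforcement-learning training for the game's tanks.
; On BeginPlay it sets up the interactor, builds the policy from it and the DA_TankNetwork asset, then passes both to the trainer.
; Tick runs training without reinitializing the policy network or resetting agents on begin.
; Disconnected logic for deriving tank count and grid size from GM_WiiTainks never runs.
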(event `self.ReceiveBeginPlay`
  (`|ExecutionSequence`
    (:`then_0`
      (`|ExecutionSequence`
        (:`then_0`
          (`LearningAgentsInteractor.SetupInteractor` (`self.BP_TankInteractor`)))
        (:`then_1`
          (`LearningAgentsPolicy.SetupPolicy` (`self.BP_TankPolicy`) (`self.BP_TankInteractor`) (`self.Policy Settings`) "/Game/Learning/DA_TankNetwork.DA_TankNetwork"))
        (:`then_2`
          (`LearningAgentsTrainer.SetupTrainer` (`self.BP_TankRLTrainer`) (`self.BP_TankInteractor`) (`self.BP_TankPolicy`) null (`self.Trainer Settings`)))))))

(event `self.ReceiveTick`
  (params (DeltaSeconds :type "Float (single-precision)"))
  (`LearningAgentsTrainer.RunTraining` (`self.BP_TankRLTrainer`) (`self.Trainer Training Settings_0`) (`self.Trainer Game Settings`) (`self.Trainer Path Settings`) (`self.Critic Settings`) false true false))

(fn `UserConstructionScript`)