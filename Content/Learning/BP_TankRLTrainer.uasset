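; Learning Agents trainer for reinforcement learning of AI tanks, defining rewards, episode completions and resets.
; Each agent's BP_TankAIController supplies weighted rewards for speed, curiosity and proximity to the nearest tank, plus a wall-contact penalty.
; Death terminates an episode, closing on another tank truncates it, and resets go through each agent's owning game container.
; Unconnected leftover nodes hold alternative rewards and completions such as turret aim, line of sight, kills and round wins.
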(event `self.SetupRewards`
  (`|ExecutionSequence`
    (:`then_0`
      (bind _returnvalue (`FloatReward.AddFloatReward` null "VelocityScalarReward" 0.5))
      (set `self.VelocityScalarReward` _returnvalue)
      (bind _returnvalue_2 (`FloatReward.AddFloatReward` null "CuriosityReward" 1.5))
      (set `self.CuriosityReward` _returnvalue_2)
      (bind _returnvalue_3 (`FloatReward.AddFloatReward` null "WallContactPenalty" -3.0))
      (set `self.WallContactPenalty` _returnvalue_3))
    (:`then_1`
      (bind _returnvalue_4 (`FloatReward.AddFloatReward` null "NearestTankProxReward" 3.0))
      (set `self.NearestTankProxReward` _returnvalue_4))))

(event `self.SetRewards`
  (params (AgentIds :type "Array of Integer (by ref)"))
  (for _array_element AgentIds
    (`|ExecutionSequence`
      (:`then_0`
        (bind _returnvalue (`self.GetAgent` _array_element "/Game/WiiTainks_Content/Tanks/Blueprints/BP_TankAIController.BP_TankAIController_C"))
        (`FloatReward.SetFloatReward` (`self.VelocityScalarReward`) _array_element (/ (`KismetMathLibrary.VSize` (`Actor.GetVelocity` (`/Game/WiiTainks_Content/Tanks/Blueprints/BP_TankAIController.Tank Pawn` _returnvalue))) (`self.Max Tank Speed`)))
        (bind _reward (`/Game/WiiTainks_Content/Tanks/Blueprints/BP_TankAIController.Get Curiosity Reward` _returnvalue))
        (`FloatReward.SetFloatReward` (`self.CuriosityReward`) _array_element _reward))
      (:`then_1`
        (bind _reward_2 (`/Game/WiiTainks_Content/Tanks/Blueprints/BP_TankAIController.GetClosestTankReward` _returnvalue))
        (`FloatReward.SetFloatReward` (`self.NearestTankProxReward`) _array_element _reward_2)
        (bind _is_in_wall_contact_ (`/Game/WiiTainks_Content/Tanks/Blueprints/BP_TankAIController.Get Is In Wall Contact?` _returnvalue))
        (`FloatReward.SetFloatReward` (`self.WallContactPenalty`) _array_element (`KismetMathLibrary.SelectFloat` 1.0 0.0 (== _is_in_wall_contact_ true)))))))

(event `self.SetupCompletions`
  (bind _returnvalue (`ConditionalCompletion.AddConditionalCompletion` null "DestroyedCompletion"))
  (set `self.DestroyedCompletion` _returnvalue)
  (bind _returnvalue_2 (`ConditionalCompletion.AddConditionalCompletion` null "TankReachedOtherTankCompletion" "Truncation"))
  (set `self.TankReachedOtherTankCompletion` _returnvalue_2))

(event `self.SetCompletions`
  (params (AgentIds :type "Array of Integer (by ref)"))
  (for _array_element AgentIds
    (`|ExecutionSequence`
      (:`then_0`
        (bind _returnvalue (`self.GetAgent` _array_element "/Game/WiiTainks_Content/Tanks/Blueprints/BP_TankAIController.BP_TankAIController_C"))
        (bind _is_deceased_ (`/Game/WiiTainks_Content/Tanks/Blueprints/BP_TankAIController.Get Death Status` _returnvalue))
        (`ConditionalCompletion.SetConditionalCompletion` (`self.DestroyedCompletion`) _array_element _is_deceased_))
      (:`then_1`
        (bind _closest_tank_distance (`/Game/WiiTainks_Content/Tanks/Blueprints/BP_TankAIController.Get Closest Tank Distance` _returnvalue))
        (bind _returnvalue_2 (< _closest_tank_distance 200.0))
        (`ConditionalCompletion.SetConditionalCompletion` (`self.TankReachedOtherTankCompletion`) _array_element _returnvalue_2)
        (if _returnvalue_2
          (`KismetSystemLibrary.PrintText` (`|FormatText` "Tanks Close Enough at {i}" _closest_tank_distance) true true (struct :`R` 1.0 :`B` 0.896126 :`A` 1.0) 15.0))))))

(event `self.ResetEpisodes`
  (params (AgentIds :type "Array of Integer (by ref)"))
  (bind _outagents (`self.GetAgents` AgentIds "/Game/WiiTainks_Content/Tanks/Blueprints/BP_TankAIController.BP_TankAIController_C"))
  (for _array_element _outagents
    (`/Game/WiiTainks_Content/Game/BP_WiiTainks_GameContainer.ResetGame` (`/Game/WiiTainks_Content/Tanks/Blueprints/BP_TankAIController.Owner Game Container` _array_element)))
  (`KismetSystemLibrary.PrintText` (`|FormatText` "RESET {i} AGENTS" (`KismetArrayLibrary.Array_Length` _outagents)) true true (struct :`R` 1.0 :`G` 0.368491 :`A` 1.0) 5.0))